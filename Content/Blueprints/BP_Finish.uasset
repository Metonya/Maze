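; BP_Finish is the level's finish trigger, marking the player as having won on reaching it.
; On BeginPlay it caches the first-person player character and every BP_Light in the level.
; When that character overlaps the Box, it sets the character's Win flag, clears the character's timer and switches all cached lights to bright green.
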(event OnComponentBeginOverlap(Box)
  (params (OverlappedComponent :type Primitive%20Component%20Object%20Reference) (OtherActor :type Actor%20Object%20Reference) (OtherComp :type Primitive%20Component%20Object%20Reference) (OtherBodyIndex :type Integer) (bFromSweep :type Boolean) (SweepResult :type Hit%20Result%20Structure%20%28by%20ref%29))
  (if (== OtherActor (Variables|Default|GetAs%20BP%20First%20Person%20Character))
    (Variables|/Game/FirstPerson/Blueprints/BP_FirstPersonCharacter.BP_FirstPersonCharacter_C|SetWin? (Variables|Default|GetAs%20BP%20First%20Person%20Character) true)
    (Utilities|Time|ClearandInvalidateTimerbyHandle (Variables|/Game/FirstPerson/Blueprints/BP_FirstPersonCharacter.BP_FirstPersonCharacter_C|GetTimerHandler (Variables|Default|GetAs%20BP%20First%20Person%20Character)))
    (for _array_element (Variables|Default|GetBP_Light)
      (Default|ChangeLightColor _array_element 8e+02 "(R=0.171800,G=1.000000,B=0.000000,A=1.000000)"))))

(event EventBeginPlay
  (bind _asbp_first_person_character (Utilities|Casting|CastToBP_FirstPersonCharacter (Game|GetPlayerCharacter 0)))
  (Variables|Default|SetAs%20BP%20First%20Person%20Character _asbp_first_person_character)
  (bind _outactors (Actor|GetAllActorsOfClass "/Game/Blueprints/BP_Light.BP_Light_C"))
  (Variables|Default|SetBP_Light _outactors))

(event Collision|EventActorBeginOverlap
  (params (OtherActor :type Actor%20Object%20Reference)))

(event EventTick
  (params (DeltaSeconds :type Float%20%28single-precision%29)))

(fn ConstructionScript)