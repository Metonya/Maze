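; BP_Start is a start trigger that begins the maze countdown when the player overlaps it.
; It caches the player on BeginPlay and uses a DoOnce so only the first player overlap starts a looping one-second timer.
; Each tick of that timer decrements Time and broadcasts the new value through MazeTime, with no stop at zero in this Blueprint.
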(event Custom|GameTime
  ;[1 1 1 0] Timer
  (bind _result (Math|Integer|DecrementInt (Variables|Default|GetTime))
    (:%20%20
      (Default|CallMazeTime _result))))

(event EventBeginPlay
  (bind _player (CallFunction|CasttoPlayer))
  (Variables|Default|SetPlayer _player))

(event Collision|EventActorBeginOverlap
  (params (OtherActor :type Actor%20Object%20Reference))
  (if (== OtherActor (Variables|Default|GetPlayer))
    (Utilities|FlowControl|DoOnce false
      (:Completed
        ;[1 1 1 0] Timer
        (bind _returnvalue (Utilities|Time|SetTimerbyEvent (delegate Custom|GameTime) 1.0 true false -1.0))
        (Variables|Default|SetGameTimer _returnvalue)))))

(fn ConstructionScript)