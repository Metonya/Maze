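; Spear trap actor that raises spears and repeatedly damages the player standing inside its box trigger.
; On player overlap, the Trap timeline lerps the spears upward while a looping timer calls Damage, which accumulates Duration and removes health roughly once per second.
; Leaving the box resets Duration and clears the timer, but does not lower the spears.
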(event OnComponentBeginOverlap(Box)
  (params (OverlappedComponent :type Primitive%20Component%20Object%20Reference) (OtherActor :type Actor%20Object%20Reference) (OtherComp :type Primitive%20Component%20Object%20Reference) (OtherBodyIndex :type Integer) (bFromSweep :type Boolean) (SweepResult :type Hit%20Result%20Structure%20%28by%20ref%29))
  (if (== OtherActor (Variables|Default|GetPlayer))
    (Variables|Default|SetDuration 0.0)
    (bind _returnvalue (Utilities|Time|SetTimerbyEvent (delegate Custom|Damage) 0.1 true))
    (Variables|Default|SetDamageAreaDuration _returnvalue)
    (bind _trap (Timeline|Trap Play)
      (:Update
        (Transformation|SetRelativeLocation (Variables|Default|GetSpearTraps) (Math|Vector|MakeVector 0.0 0.0 (Math|Float|Lerp -2.5e+02 -5e+01 _trap)) false false)))))

(event OnComponentEndOverlap(Box)
  (params (OverlappedComponent :type Primitive%20Component%20Object%20Reference) (OtherActor :type Actor%20Object%20Reference) (OtherComp :type Primitive%20Component%20Object%20Reference) (OtherBodyIndex :type Integer))
  (if (== OtherActor (Variables|Default|GetPlayer))
    (Variables|Default|SetDuration 0.0)
    (Utilities|Time|ClearandInvalidateTimerbyHandle (Variables|Default|GetDamageAreaDuration))))

(event Custom|Damage
  (if (>= (Variables|Default|GetDuration) 1.0)
    (Default|UpdateHealth (Variables|Default|GetPlayer) -20)
    (Variables|Default|SetDuration 0.0)
    (CallFunction|Damage)
    (else
      (Variables|Default|SetDuration (+ (Variables|Default|GetDuration) 0.1)))))

(event EventBeginPlay
  (bind _player (CallFunction|CasttoPlayer))
  (Variables|Default|SetPlayer _player))

(fn ConstructionScript)