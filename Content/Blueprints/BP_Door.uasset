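; A color-coded locked door that opens when the player character's inventory holds the key matching its Color.
; The construction script tints the door material from a color lookup, and a box overlap starts and ends the player's interact line traces.
; Focusing the closed door briefly shows an open or key-error prompt.
; PickUp rechecks the key, then a one-shot timeline swings the Sphere pivot open and clears the text.
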(event OnComponentEndOverlap(Box)
  (params (OverlappedComponent :type Primitive%20Component%20Object%20Reference) (OtherActor :type Actor%20Object%20Reference) (OtherComp :type Primitive%20Component%20Object%20Reference) (OtherBodyIndex :type Integer))
  (bind _as_bp_first_person_character (Variables|Default|GetAs%20BP%20First%20Person%20Character))
  ;[1 1 1] Alandan Çıkarsa Etkileşimi Bitir
  (if (== OtherActor _as_bp_first_person_character)
    (Default|EndInteractLines _as_bp_first_person_character)))

(event OnComponentBeginOverlap(Box)
  (params (OverlappedComponent :type Primitive%20Component%20Object%20Reference) (OtherActor :type Actor%20Object%20Reference) (OtherComp :type Primitive%20Component%20Object%20Reference) (OtherBodyIndex :type Integer) (bFromSweep :type Boolean) (SweepResult :type Hit%20Result%20Structure%20%28by%20ref%29))
  (bind _as_bp_first_person_character (Variables|Default|GetAs%20BP%20First%20Person%20Character))
  ;[1 1 1] Ray
  (if (== OtherActor _as_bp_first_person_character)
    (Default|StartInteractLines _as_bp_first_person_character)))

(event EventBeginPlay
  (bind _asbp_first_person_character (Utilities|Casting|CastToBP_FirstPersonCharacter (Game|GetPlayerCharacter 0)))
  (Variables|Default|SetAs%20BP%20First%20Person%20Character _asbp_first_person_character))

(event EventPickUp
  (bind _sphere (Variables|Default|GetSphere))
  (bind _returnvalue (Transformation|GetWorldRotation _sphere))
  ;[1 1 1] PickUp
  (bind _key (CallFunction|CheckKey))
  (if _key
    (Utilities|FlowControl|DoOnce false
      (:Completed
        (Variables|Default|SetIsOpened true)
        (bind _dooropening (Timeline|Open%20Door Play)
          (:Update
            (Transformation|SetRelativeRotation _sphere (Math|Rotator|MakeRotator (.roll _returnvalue) (.pitch _returnvalue) (Math|Float|Lerp 0.0 -9e+01 _dooropening)) false false)
            ;[1 1 1] On Focus Object Press E Text
            (Rendering|Components|TextRender|SetText (Variables|Default|GetTextRender) (Utilities|Text|FormatText ""))))))))

(event EventOnFocusObject
  ;[1 1 1] On Focus Object Press E Text
  (if (not (Variables|Default|GetIsOpened))
    (bind _key (CallFunction|CheckKey))
    (if _key
      (Rendering|Components|TextRender|SetText (Variables|Default|GetTextRender) (Variables|Default|GetOpenDoor))
      (else
        (Rendering|Components|TextRender|SetText (Variables|Default|GetTextRender) (Variables|Default|GetKeyError))))
    (Utilities|FlowControl|Delay 2.0)
    (Rendering|Components|TextRender|SetText (Variables|Default|GetTextRender) (Utilities|Text|FormatText ""))))

(fn ConstructionScript
  (bind _door (Variables|Default|GetDoor))
  ;[1 1 1] Kapı Rengi
  (bind _returnvalue (Rendering|Material|CreateDynamicMaterialInstance _door 2 (Rendering|Material|GetMaterial _door 2) "None" :!class /Script/Engine.PrimitiveComponent))
  (Rendering|Material|SetVectorParameterValue _returnvalue "SurfaceColor" (.Value (Utilities|Map|Find (Variables|Default|GetColorList) (Utilities|String|EnumtoString (Variables|Default|GetColor)))) :!class /Script/Engine.MaterialInstanceDynamic))

(fn CheckKey
  (if (!= (Utilities|Array|FindItem (Variables|/Game/FirstPerson/Blueprints/BP_FirstPersonCharacter.BP_FirstPersonCharacter_C|GetInventory (Variables|Default|GetAs%20BP%20First%20Person%20Character)) (Utilities|String|EnumtoString (Variables|Default|GetColor))) -1)
    (return true)
    (else
      (return false))))