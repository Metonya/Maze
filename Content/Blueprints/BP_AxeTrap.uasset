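; BP_AxeTrap is a swinging axe hazard that damages the player when triggered by a trap wire.
; On BeginPlay it caches the player and binds to the activation event of the first BP_TrapWire found in the level.
; Activation plays a timeline that swings the Sphere component's pitch through 180 degrees.
; Axe hits pass through a DoOnce, which resets after a short delay only when the player was hit.
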(event OnComponentHit(Axe_Double)
  (params (HitComponent :type Primitive%20Component%20Object%20Reference) (OtherActor :type Actor%20Object%20Reference) (OtherComp :type Primitive%20Component%20Object%20Reference) (NormalImpulse :type Vector :default "0, 0, 0") (Hit :type Hit%20Result%20Structure%20%28by%20ref%29))
  (Utilities|FlowControl|DoOnce false :!label _label
    (:Completed
      (if (== OtherActor (Variables|Default|GetPlayer))
        (Default|UpdateHealth (Variables|Default|GetPlayer) -20)
        (Utilities|FlowControl|Delay 1.0)
        (goto _label Reset)))))

(event Custom|Activate%20Trap
  (bind _rotation (Variables|Default|GetRotation))
  (bind _trap (Timeline|Trap Play)
    (:Update
      (Transformation|SetRelativeRotation (Variables|Default|GetSphere) (Math|Rotator|MakeRotator 0.0 (Math|Float|Lerp (.pitch _rotation) (- (.pitch _rotation) 1.8e+02) _trap) 0.0) false false))))

(event EventBeginPlay
  (bind _player (CallFunction|CasttoPlayer))
  (Variables|Default|SetPlayer _player)
  (bind _outactors (Actor|GetAllActorsOfClass "/Game/Blueprints/BP_TrapWire.BP_TrapWire_C"))
  (bind _asbp_trap_wire (Utilities|Casting|CastToBP_TrapWire (Utilities|Array|Get(acopy) _outactors)))
  (EventDispatchers|BindEventtoActivateAxeTrap _asbp_trap_wire (delegate Custom|Activate%20Trap)))

(fn ConstructionScript)