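; Base collectable the first-person character picks up, either a colored item added to the inventory or gold worth a random price.
; An overlap box starts and ends the character's interact lines, and focusing briefly shows a prompt widget.
; The construction script tints meshes from the Color enum via dynamic materials, stacking extra cones for higher gold prices or configuring mesh and InterpToMovement for other colors.
; Pickup adds gold or the color name, then destroys the actor.
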(event OnComponentBeginOverlap(Box)
  (params (OverlappedComponent :type Primitive%20Component%20Object%20Reference) (OtherActor :type Actor%20Object%20Reference) (OtherComp :type Primitive%20Component%20Object%20Reference) (OtherBodyIndex :type Integer) (bFromSweep :type Boolean) (SweepResult :type Hit%20Result%20Structure%20%28by%20ref%29))
  (bind _as_bp_first_person_character (Variables|Default|GetAs%20BP%20First%20Person%20Character))
  ;[1 1 1] Ray
  (if (== OtherActor _as_bp_first_person_character)
    (Default|StartInteractLines _as_bp_first_person_character)))

(event OnComponentEndOverlap(Box)
  (params (OverlappedComponent :type Primitive%20Component%20Object%20Reference) (OtherActor :type Actor%20Object%20Reference) (OtherComp :type Primitive%20Component%20Object%20Reference) (OtherBodyIndex :type Integer))
  (bind _as_bp_first_person_character (Variables|Default|GetAs%20BP%20First%20Person%20Character))
  ;[1 1 1] Alandan Çıkarsa Etkileşimi Bitir
  (if (== OtherActor _as_bp_first_person_character)
    (Default|EndInteractLines _as_bp_first_person_character)))

(event EventBeginPlay
  (bind _asbp_first_person_character (Utilities|Casting|CastToBP_FirstPersonCharacter (Game|GetPlayerCharacter 0)))
  (Variables|Default|SetAs%20BP%20First%20Person%20Character _asbp_first_person_character))

(event EventPickUp
  (bind _as_bp_first_person_character (Variables|Default|GetAs%20BP%20First%20Person%20Character))
  ;[1 1 1] PickUp
  (if (Utilities|Enum|NotEqual(Enum) (Utilities|String|EnumtoString (Variables|Default|GetColor)) "Gold")
    (Utilities|Array|Add (Variables|/Game/FirstPerson/Blueprints/BP_FirstPersonCharacter.BP_FirstPersonCharacter_C|GetInventory (Variables|Default|GetAs%20BP%20First%20Person%20Character)) (Utilities|String|EnumtoString (Variables|Default|GetColor)))
    (Actor|DestroyActor)
    (else
      (Variables|/Game/FirstPerson/Blueprints/BP_FirstPersonCharacter.BP_FirstPersonCharacter_C|SetGold _as_bp_first_person_character (+ (Variables|Default|GetPrice) (Variables|/Game/FirstPerson/Blueprints/BP_FirstPersonCharacter.BP_FirstPersonCharacter_C|GetGold _as_bp_first_person_character)))
      (Actor|DestroyActor))))

(event EventOnFocusObject
  ;[1 1 1] On Focus Object Press E Text
  (Rendering|SetVisibility (Variables|Default|GetWidget) true false)
  (Utilities|FlowControl|Delay 2.0)
  (Rendering|SetVisibility (Variables|Default|GetWidget) false false))

(fn ConstructionScript
  (bind _collectable (Variables|Default|GetCollectable))
  (if (Utilities|Enum|Equal(Enum) (Utilities|String|EnumtoString (Variables|Default|GetColor)) "Gold")
    (Variables|Default|SetPrice (Math|Random|RandomIntegerinRange 1 99))
    ;[1 1 1] Gold Base
    (Components|StaticMesh|SetStaticMesh (Variables|Default|GetCollectable) "/Game/Blueprints/SM_Cone.SM_Cone")
    (CallFunction|ChangeColor (Variables|Default|GetCollectable))
    ;[1 1 1] Cone2
    (if (>= (Variables|Default|GetPrice) 26)
      (bind _returnvalue (AddComponent|AddStaticMeshComponent false (Math|Transform|MakeTransform "-50.000000,80.000000,-25.000000" "0, 0, 0" "0.500000,0.500000,0.500000")))
      (CallFunction|ChangeColor _returnvalue)
      ;[1 1 1] Cone3
      (if (>= (Variables|Default|GetPrice) 76)
        (bind _returnvalue_2 (AddComponent|AddStaticMeshComponent false (Math|Transform|MakeTransform "-80.000000,40.000000,-37.000000" "0, 0, 0" "0.250000,0.250000,0.250000")))
        (CallFunction|ChangeColor _returnvalue_2)))
    (else
      ;[1 1 1] Değiştirilebilir Mesh
      (Components|StaticMesh|SetStaticMesh (Variables|Default|GetCollectable) (Variables|Default|GetMesh))
      ;[1 1 1] Interp
      (Components|Activation|SetAutoActivate (Variables|Default|GetInterpToMovement) (Variables|Interp|GetInterpActivation))
      (Variables|/Script/Engine.InterpToMovementComponent|SetDuration (Variables|Default|GetInterpToMovement) (Variables|Interp|GetInterpDuration))
      (Class|InterptoMovementComponent|AddControlPointPosition (Variables|Default|GetInterpToMovement) (Variables|Interp|GetInterpPos1) true)
      (Class|InterptoMovementComponent|AddControlPointPosition (Variables|Default|GetInterpToMovement) (Variables|Interp|GetInterpPos2) true)
      ;[1 1 1] Değiştirilebilir Renk
      (bind _returnvalue_3 (Rendering|Material|CreateDynamicMaterialInstance _collectable 0 (Rendering|Material|GetMaterial _collectable 0) "None" :!class /Script/Engine.PrimitiveComponent))
      (Rendering|Material|SetVectorParameterValue _returnvalue_3 "SurfaceColor" (.Value (Utilities|Map|Find (Variables|Default|GetColorList) (Utilities|String|EnumtoString (Variables|Default|GetColor)))) :!class /Script/Engine.MaterialInstanceDynamic))))

(fn ChangeColor
  (params (Target :type Primitive%20Component%20Object%20Reference))
  ;[1 1 1] Değiştirilebilir Renk
  (bind _returnvalue (Rendering|Material|CreateDynamicMaterialInstance Target 0 (Rendering|Material|GetMaterial Target 0) "None" :!class /Script/Engine.PrimitiveComponent))
  (Rendering|Material|SetVectorParameterValue _returnvalue "SurfaceColor" (.Value (Utilities|Map|Find (Variables|Default|GetColorList) (Utilities|String|EnumtoString (Variables|Default|GetColor)))) :!class /Script/Engine.MaterialInstanceDynamic))