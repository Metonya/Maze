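; BP_MazeCell is a modular maze cell actor that builds its geometry in the construction script from a GridSize value.
; It scales the floor, then reads DT_Wall rows to add wall meshes at stored transforms for sides enabled in the Walls map.
; After the first wall, a DoOnce adds an optional roof with a light child actor.
; SizeToCubeScale converts dimensions into cube mesh scale.
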(event EventBeginPlay)

(event Collision|EventActorBeginOverlap
  (params (OtherActor :type Actor%20Object%20Reference)))

(event EventTick
  (params (DeltaSeconds :type Float%20%28single-precision%29)))

(fn ConstructionScript
  (bind _gridsize (Variables|Default|GetGridSize))
  ;[1 1 1] Zemin
  (Variables|Default|SetWallHeight _gridsize)
  (Variables|Default|SetWallTickness (* _gridsize 0.1))
  (Transformation|SetRelativeScale3D (Variables|Default|GetFloor) (Utilities|SizetoCubeScale (Math|Vector|MakeVector (Variables|Default|GetWallHeight) (Variables|Default|GetWallHeight) (Variables|Default|GetWallTickness))))
  ;[1 1 1] DataTable'daki Her Satır için
  (bind _outrownames (DataTable|GetDataTableRowNames "/Game/Blueprints/Data/DT_Wall.DT_Wall"))
  (for _array_element _outrownames
    ;[1 1 1] DT_Wall'dan gelen lokasyon ve rotasyon bilgisine göre ve o duvarın oluşup oluşmayacağına göre static mesh spawn edicek
    (bind _returnvalue (Utilities|GetDataTableRow "/Game/Blueprints/Data/DT_Wall.DT_Wall" _array_element)
      (:then
        (if (.Value (Utilities|Map|Find (Variables|Default|GetWalls) (.Name (Utilities|Struct|BreakS_Wall _returnvalue))))
          (AddComponent|AddStaticMeshComponent false (Math|Transform|MakeTransform (.Location (Utilities|Struct|BreakS_Wall _returnvalue)) (.Rotation (Utilities|Struct|BreakS_Wall _returnvalue)) (Utilities|SizetoCubeScale (Math|Vector|MakeVector (Variables|Default|GetWallTickness) (Variables|Default|GetWallHeight) (Variables|Default|GetWallHeight)))))
          ;[1 1 1] Çatı?
          (Utilities|FlowControl|DoOnce false
            (:Completed
              (if (Variables|Default|GetRoof)
                (AddComponent|AddStaticMeshComponent false (Math|Transform|MakeTransform "0.000000,0.000000,550.000000" "0, 0, 0" (Utilities|SizetoCubeScale (Math|Vector|MakeVector (Variables|Default|GetWallHeight) (Variables|Default|GetWallHeight) (Variables|Default|GetWallTickness)))))
                ;[1 1 1] Light
                (AddComponent|AddChildActorComponent false (Math|Transform|MakeTransform "250.000000,250.000000,550.000000" "0, 0, 0" "0.100000,0.100000,0.100000"))))))))))